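; Moving actor that shuttles back and forth between two target positions along a single axis, X or Z as chosen by MoveXZ.
; Each Tick calls Move, which teleports the actor toward the current target at a speed proportional to remaining distance, easing out and snapping when close.
; Once Move reports arrival, Tick swaps Target1 and Target2; each teleport also resets rotation to zero.
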(event `self.ReceiveBeginPlay`
  (set `self.TempTarget` (`self.Target1`)))

(event `self.ReceiveTick`
  (params (DeltaSeconds :type "Float (single-precision)"))
  (bind _is_reach (`self.Move` DeltaSeconds (`self.MoveXZ`) self (`self.TempTarget`)))
  (if _is_reach
    (if (== (`self.Target1`) (`self.TempTarget`) :`ErrorTolerance` 0.01)
      (set `self.TempTarget` (`self.Target2`))
      (else
        (set `self.TempTarget` (`self.Target1`))))))

(fn `Move`
  (params (DeltaSeconds :type "Float (double-precision)") (MoveXZ :type Boolean) (Actorreference :type "Actor Object Reference") (Target :type "Vector Structure"))
  (returns (`is reach` :type Boolean))
  (locals (isXZ :type Boolean) (ActorRef :type "Actor Object Reference") (DeltaSec :type "Float (double-precision)") (`Real Target` :type "Vector Structure") (`Linear Target` :type "Float (double-precision)") (Linearorigin :type "Float (double-precision)") (snap :type Boolean) (OriginalTarget :type "Vector Structure") (Speed :type "Float (double-precision)") (NextZone :type "Vector Structure"))
  (bind (_originaltarget_x _originaltarget_y _originaltarget_z) (`KismetMathLibrary.BreakVector` (`local.OriginalTarget`)))
  (bind _linear_target (`local.Linear Target`))
  (bind _linearorigin (`local.Linearorigin`))
  (bind (_returnvalue_x _returnvalue_y _returnvalue_z) (`KismetMathLibrary.BreakVector` (`self.K2_GetActorLocation` (`local.ActorRef`))))
  (bind (_returnvalue_x_2 _returnvalue_y_2 _returnvalue_z_2) (`KismetMathLibrary.BreakVector` (`self.K2_GetActorLocation` (`local.ActorRef`))))
  (bind _returnvalue (+ (* (`local.DeltaSec`) (`local.Speed`)) (`local.Linearorigin`)))
  (set `local.DeltaSec` DeltaSeconds)
  (set `local.isXZ` MoveXZ)
  (set `local.ActorRef` Actorreference)
  (set `local.OriginalTarget` Target)
  (if (`local.isXZ`)
    (set `local.Linearorigin` _returnvalue_x)
    (set `local.Real Target` (`KismetMathLibrary.MakeVector` _originaltarget_x _returnvalue_y _returnvalue_z))
    (set `local.Linear Target` _originaltarget_x)
    (else
      (set `local.Linearorigin` _returnvalue_z)
      (set `local.Real Target` (`KismetMathLibrary.MakeVector` _returnvalue_x _returnvalue_y _originaltarget_z))
      (set `local.Linear Target` _originaltarget_z)))
  (bind _output_get (set `local.Speed` (* (- _linear_target _linearorigin) 2.0)))
  (if (<= (`KismetMathLibrary.Abs` _output_get) 1.0)
    (set `local.snap` true)
    (else
      (set `local.snap` false)))
  (if (== _linear_target _linearorigin)
    (return true)
    (else
      (if (`local.snap`)
        (set `local.NextZone` (`local.Real Target`))
        (elif (`local.isXZ`)
          (set `local.NextZone` (`KismetMathLibrary.MakeVector` _returnvalue _returnvalue_y_2 _returnvalue_z_2))
          (else
            (set `local.NextZone` (`KismetMathLibrary.MakeVector` _returnvalue_x_2 _returnvalue_y_2 _returnvalue)))))
      (`self.K2_TeleportTo` :`self` (`local.ActorRef`) :`DestLocation` (`local.NextZone`))
      (return false))))

(fn `UserConstructionScript`)