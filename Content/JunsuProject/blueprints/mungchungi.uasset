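; Actor Blueprint for an apparent mover meant to shuttle between Target and Target2 along one axis, still unfinished.
; Tick calls Move It, which only builds a temporary target from RealTarget on X or Z, chosen by MoveXZ.
; The stepping, snap, Teleport and FlipFlop target swap are disconnected and never run, so the actor stays still.
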(event `self.ReceiveBeginPlay`
  (set `self.real target` (`self.target`)))

(event `self.ReceiveTick`
  (params (DeltaSeconds :type "Float (single-precision)"))
  (`self.Move It` DeltaSeconds (`self.MoveXZ`) self))

(fn `Move It`
  (params (DeltaSeconds :type "Float (double-precision)") (MoveXZ :type Boolean) (`Reference To Actor` :type "Actor Object Reference"))
  (locals (`Is XZ` :type Boolean) (`Linear Target` :type "Float (double-precision)") (`Linear origin` :type "Float (double-precision)") (SnapV :type Boolean))
  (bind _returnvalue (`self.GetTransform` `Reference To Actor`))
  (bind (_real_target_x _real_target_y _real_target_z) (`KismetMathLibrary.BreakVector` (`self.real target`)))
  (bind _output_get (set `local.Is XZ` MoveXZ))
  (if _output_get
    (set `self.TempTarget` (`KismetMathLibrary.MakeVector` (.x (.location _returnvalue)) (.y (.location _returnvalue)) _real_target_z))
    (else
      (set `self.TempTarget` (`KismetMathLibrary.MakeVector` _real_target_x (.y (.location _returnvalue)) (.z (.location _returnvalue)))))))

(fn `UserConstructionScript`)